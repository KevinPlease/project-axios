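; Master tile Blueprint that has obstacles spawned on it and awards points to players who cross it.
; On BeginPlay it passes its Left, Center and Right references to GM_Gameplay's SpawnObstacles, flagging a skip while InitialCount is below two.
; Box overlaps by BP_Character_Gameplay score through the game mode, ignoring repeats from the last stored player controller.
; IsInGame reports whether the game mode's GameOver flag is unset.
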(event OnComponentBeginOverlap(Box)
  (params (OverlappedComponent :type Primitive%20Component%20Object%20Reference) (OtherActor :type Actor%20Object%20Reference) (OtherComp :type Primitive%20Component%20Object%20Reference) (OtherBodyIndex :type Integer) (bFromSweep :type Boolean) (SweepResult :type Hit%20Result%20Structure%20%28by%20ref%29))
  ;[1 1 1] Add points to the collapsed player controller
  (bind _asbp_character_gameplay (Utilities|Casting|CastToBP_Character_Gameplay OtherActor))
  (bind _asplayer_controller (Utilities|Casting|CastToPlayerController (Pawn|GetController _asbp_character_gameplay)))
  (if (!= _asplayer_controller (Variables|Default|GetPlayerControllerRef))
    (bind _output_get (Variables|Default|SetPlayerControllerRef _asplayer_controller))
    (Default|PointScoreforPlayer (Variables|References|GetGameModeRef) _output_get)))

(event EventBeginPlay
  ;[1 1 1] Begin Play
  (bind _asgm_gameplay (Utilities|Casting|CastToGM_Gameplay (Game|GetGameMode)))
  (Variables|References|SetGameModeRef _asgm_gameplay)
  (Default|SpawnObstacles (Variables|References|GetGameModeRef) (Variables|Default|GetLeft) (Variables|Default|GetCenter) (Variables|Default|GetRight) (< (Variables|/Game/Blueprints/Gameplay/GM_Gameplay.GM_Gameplay_C|GetInitialCount (Variables|References|GetGameModeRef)) 2)))

(fn ConstructionScript)

(fn IsinGame
  (return (not (Variables|/Game/Blueprints/Gameplay/GM_Gameplay.GM_Gameplay_C|GetGameOver (Variables|References|GetGameModeRef)))))