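; Playable runner character that moves forward every tick, steers, jumps, slams down mid-air and shoves other runners.
; Touch swipes (up/down only) and keys drive actions, with Z/X starting left/right pushes.
; After a montage delay, pushes check a capsule-overlapped character's Y side, then temporarily scale the victim's walk speed by push force.
; Death disables movement, sets UI-only input and saves high scores; a helper updates the HUD countdown.
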(event Custom|Event%20Pushed
  (params (Pushed%20From :type Name) (Push%20Force :type Float%20%28single-precision%29))
  (bind _charactermovement (Variables|Character|GetCharacterMovement))
  ;[1 1 1] Push this actor by an offset vector multiplied by a push force
  (Animation|PlayAnimMontage "/Game/Characters/Animations/Female/AnimMontage_Female_Pushed.AnimMontage_Female_Pushed" 1.0 (CallFunction|GetAnimName Pushed%20From))
  (Variables|MyCharacter|SetCharacterWalkSpeed (Variables|/Script/Engine.CharacterMovementComponent|GetMaxWalkSpeed _charactermovement))
  (Variables|/Script/Engine.CharacterMovementComponent|SetMaxWalkSpeed _charactermovement (* Push%20Force (Variables|MyCharacter|GetCharacterWalkSpeed)))
  (Utilities|FlowControl|Delay 0.7)
  (Variables|/Script/Engine.CharacterMovementComponent|SetMaxWalkSpeed _charactermovement (Variables|MyCharacter|GetCharacterWalkSpeed)))

(event Custom|Begin%20Push
  (params (Left%20or%20RIght :type Integer))
  ;[1 1 1] Push Character - Play Animation & Check for actors to push
  (switch int Left%20or%20RIght
    (:0
      (Variables|MyCharacter|SetPushDirection "Push_Left"))
    (:1
      (Variables|MyCharacter|SetPushDirection "Push_Right")))
  (Animation|PlayAnimMontage "/Game/Characters/Animations/Female/AnimMontage_Female_Push.AnimMontage_Female_Push" 1.0 (Variables|MyCharacter|GetPushDirection))
  (Utilities|FlowControl|Delay 0.7)
  (CallFunction|PushOverlappingActor))

(event Custom|CharacterDeath
  (params (Simulate%20Physics :type Boolean))
  ;[1 1 1] Disable Character on Game Over
  ;;[1 1 1] Death Anim. purposes
  (Physics|SetSimulatePhysics (Variables|Character|GetMesh) Simulate%20Physics)
  (Pawn|Components|CharacterMovement|DisableMovement (Variables|Character|GetCharacterMovement))
  (Input|SetInputModeUIOnly (Game|GetPlayerController 0) 0 "DoNotLock")
  (CallFunction|GameOverSave))

(event EventTick
  (params (DeltaSeconds :type Float%20%28single-precision%29))
  ;[1 1 1] Movement input - Checks if in gameplay and splits movement logic vs "swipe to move"
  (Pawn|Input|AddMovementInput (Math|Vector|GetForwardVector (Math|Rotator|MakeRotator 0.0 0.0 (.Yaw (Math|Rotator|BreakRotator (Pawn|GetControlRotation :!class /Script/Engine.Pawn))))) 1.0 false))

(event EventBeginPlay
  (bind _returnvalue (Game|GetPlayerController 0))
  ;[1 1 1] Get Refs
  (bind _aspc_gameplay (Utilities|Casting|CastToPC_Gameplay _returnvalue)
    (:then
      (bind _output_get (Variables|References|SetPlayerControllerRef _aspc_gameplay))
      (Variables|References|SetGameplayHUD (Variables|/Game/Blueprints/Gameplay/PC_Gameplay.PC_Gameplay_C|GetGameplayHUD _output_get)))
    (:CastFailed
      (bind _asgm_gameplay (Utilities|Casting|CastToGM_Gameplay (Game|GetGameMode)))
      (Variables|References|SetGameModeRef _asgm_gameplay)))
  (Input|SetInputModeUIOnly _returnvalue 0 "DoNotLock"))

(event Input|ActionEvents|InputActionJump
  (params (Key :type Key%20Structure :default "None"))
  ;[1 1 1] Keyboard Input - Jump
  (:Pressed
    (Character|Jump)))

(event Input|AxisEvents|InputAxisMoveRight
  (params (AxisValue :type Float%20%28single-precision%29))
  ;[1 1 1] Movement input - Checks if in gameplay and splits movement logic vs "swipe to move"
  (Pawn|Input|AddMovementInput (Math|Vector|GetRightVector (Math|Rotator|MakeRotator 0.0 0.0 (.Yaw (Math|Rotator|BreakRotator (Pawn|GetControlRotation :!class /Script/Engine.Pawn))))) AxisValue false))

(event Input|AxisEvents|InputAxisMoveForward
  (params (AxisValue :type Float%20%28single-precision%29))
  ;[1 1 1] Movement input - Checks if in gameplay and splits movement logic vs "swipe to move"
  (if (not (Variables|Gameplay|GetIsInGameplay))
    (Pawn|Input|AddMovementInput (Math|Vector|GetForwardVector (Math|Rotator|MakeRotator 0.0 0.0 (.Yaw (Math|Rotator|BreakRotator (Pawn|GetControlRotation :!class /Script/Engine.Pawn))))) AxisValue false)))

(event Input|KeyboardEvents|X
  (params (Key :type Key%20Structure :default "None"))
  ;[1 1 1] Keyboard Input for Pushing Left/Right
  (:Pressed
    (CallFunction|BeginPush 1)))

(event Input|KeyboardEvents|Z
  (params (Key :type Key%20Structure :default "None"))
  ;[1 1 1] Keyboard Input for Pushing Left/Right
  (:Pressed
    (CallFunction|BeginPush)))

(event Input|KeyboardEvents|Down
  (params (Key :type Key%20Structure :default "None"))
  (bind _charactermovement (Variables|Character|GetCharacterMovement))
  ;[1 1 1] Keyboard Input - Push down to the ground if in air
  (:Pressed
    (if (AI|Components|NavMovement|IsFalling _charactermovement)
      (Physics|AddImpulse _charactermovement "0, 0,-3000.000000" true))))

(event Input|TouchEvents|InputTouch
  (params (Location :type Vector) (FingerIndex :type ETouchIndex%20Enum))
  (bind _returnvalue (CallFunction|GetTouchLocation))
  (bind _charactermovement (Variables|Character|GetCharacterMovement))
  ;[1 1 1] Swipe Controls
  (:Pressed
    (Variables|Controls|SetIsPressed true)
    (Variables|Controls|SetTouchStart2D _returnvalue))
  (:Released
    (Variables|Controls|SetIsPressed false)
    (if (> (Math|Vector2D|Vector2DLength (- (Variables|Controls|GetTouchStart2D) _returnvalue)) 1e+02)
      (Utilities|FlowControl|Sequence
        (:then_0
          (Utilities|FlowControl|DoOnce false :!label _label
            (:Completed
              (Variables|Controls|SetTouchEnd2D _returnvalue)
              (switch string (CallFunction|GetFinalSwipeDirection (Variables|Controls|GetTouchStart2D) (Variables|Controls|GetTouchEnd2D))
                (:Up
                  (Character|Jump))
                (:Down
                  (if (AI|Components|NavMovement|IsFalling _charactermovement)
                    (Physics|AddImpulse _charactermovement "0, 0,-3000.000000" true)))))))
        (:then_1
          (Utilities|FlowControl|Delay 0.5)
          (goto _label Reset))))))

(fn ConstructionScript)

(fn GetMyGameMode
  (Utilities|IsValid (Variables|References|GetGameModeRef)
    (:Is%20Valid
      _)
    (:Is%20Not%20Valid
      (bind _asgm_gameplay (Utilities|Casting|CastToGM_Gameplay (Game|GetGameMode)))
      (Variables|References|SetGameModeRef _asgm_gameplay)))
  (return (Variables|References|GetGameModeRef)))

(fn PushOverlappingActor
  ;[1 1 1] Check for valid character in radius && Compare location to find direction of push && Commit push
  (bind _asbp_character_gameplay (Utilities|Casting|CastToBP_Character_Gameplay (Utilities|Array|Get(acopy) (Collision|GetOverlappingActors (Variables|Default|GetPushCapsule) "BP_Character_Gameplay_C" :!class /Script/Engine.PrimitiveComponent) 1)))
  (Math|Float|CompareFloat (.y (Transformation|GetActorLocation _asbp_character_gameplay)) (.y (Transformation|GetActorLocation))
    (:>
      (LocalVariables|SetPushedActorLocation "Push_Right"))
    (:<
      (LocalVariables|SetPushedActorLocation "Push_Left")))
  (if (Utilities|Enum|Equal(Enum) (LocalVariables|GetPushedActorLocation) (Utilities|String|ToString(Name) (Variables|MyCharacter|GetPushDirection)))
    (CallFunction|EventPushed _asbp_character_gameplay (Variables|MyCharacter|GetPushDirection) (Variables|Stats|GetStatPushForce))))

(fn GetTouchLocation
  (bind _returnvalue (Game|GetPlayerController 0))
  (bind (_locationx _locationy) (Class|PlayerController|GetInputTouchState _returnvalue "Touch1"))
  (return (Math|Vector2D|MakeVector2D _locationx _locationy)))

(fn GetFinalSwipeDirection
  (params (TouchStart :type Vector%202D%20Structure) (TouchEnd :type Vector%202D%20Structure))
  (bind _returnvalue (- TouchStart TouchEnd))
  (if (> (Math|Float|Absolute(Float) (.x _returnvalue)) (Math|Float|Absolute(Float) (.y _returnvalue)))
    (if (> (.x _returnvalue) 0.0)
      (LocalVariables|SetSwipeDir "Left")
      (else
        (LocalVariables|SetSwipeDir "Right")))
    (elif (> (.y _returnvalue) 0.0)
      (LocalVariables|SetSwipeDir "Up")
      (else
        (LocalVariables|SetSwipeDir "Down"))))
  (return (LocalVariables|GetSwipeDir)))

(fn GetAnimName
  (params (From%20Push%20Anim%20Name :type Name))
  (switch name From%20Push%20Anim%20Name
    (:Push_Left
      (LocalVariables|SetAnim%20Montage "Pushed_From_Left"))
    (:Push_Right
      (LocalVariables|SetAnim%20Montage "Pushed_From_Right")))
  (return (LocalVariables|GetAnim%20Montage)))

(fn UpdateCountdown
  (params (TimeRemaining :type Float%20%28single-precision%29))
  (bind _gameplayhud (Variables|References|GetGameplayHUD))
  (bind _text_counter (Variables|/Game/UI/Blueprints/Gameplay/WB_MainHUD.WB_MainHUD_C|GetText_Counter _gameplayhud))
  (LocalVariables|SetRemTime TimeRemaining)
  (Utilities|IsValid _text_counter
    (:Is%20Valid
      (Rendering|Components|TextRender|SetText _text_counter (Utilities|Text|ToText(Float) (LocalVariables|GetRemTime) "HalfToEven" false true 1 324 0 0))
      (if (== (LocalVariables|GetRemTime) 0.0)
        (Widget|SetVisibility _text_counter "Collapsed")))))

(fn GameOverSave
  (bind _playercontrollerref (Variables|References|GetPlayerControllerRef))
  (bind _scoredpoints (Variables|/Game/Blueprints/Gameplay/PC_Gameplay.PC_Gameplay_C|GetScoredPoints _playercontrollerref))
  (bind _returnvalue (SaveGame|DoesSaveGameExist (Variables|Gameplay|GetSlotName)))
  (if _returnvalue
    ;[1 1 1] Load Game and Highscore
    (bind _returnvalue_2 (SaveGame|LoadGamefromSlot (Variables|Gameplay|GetSlotName)))
    (bind _asbp_runner_save_game (Utilities|Casting|CastToBP_RunnerSaveGame _returnvalue_2))
    (bind _output_get (Variables|References|SetSaveGameRef _asbp_runner_save_game))
    (if (< (Variables|/Game/Blueprints/AllLevels/BP_RunnerSaveGame.BP_RunnerSaveGame_C|GetHighScore _output_get) _scoredpoints)
      (bind _output_get_2 (Variables|/Game/Blueprints/AllLevels/BP_RunnerSaveGame.BP_RunnerSaveGame_C|SetHighScore (Variables|References|GetSaveGameRef) _scoredpoints))
      (LocalVariables|SetPointsToShow _output_get_2)
      (SaveGame|SaveGametoSlot (Variables|References|GetSaveGameRef) (Variables|Gameplay|GetSlotName))
      (else
        (LocalVariables|SetPointsToShow (Variables|/Game/Blueprints/AllLevels/BP_RunnerSaveGame.BP_RunnerSaveGame_C|GetHighScore _output_get))))
    (else
      ;[1 1 1] Create new Savegame and set highscore.
      (bind _returnvalue_3 (SaveGame|CreateSaveGameObject "/Game/Blueprints/AllLevels/BP_RunnerSaveGame.BP_RunnerSaveGame_C"))
      (bind _output_get_3 (Variables|References|SetSaveGameRef _returnvalue_3))
      (bind _output_get_4 (Variables|/Game/Blueprints/AllLevels/BP_RunnerSaveGame.BP_RunnerSaveGame_C|SetHighScore _output_get_3 _scoredpoints))
      (LocalVariables|SetPointsToShow _output_get_4)
      (SaveGame|SaveGametoSlot _output_get_3 (Variables|Gameplay|GetSlotName)))))