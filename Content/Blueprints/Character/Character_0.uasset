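; Character Blueprint that lets a character push others and react to being pushed.
; BeginPush plays the left or right section of a push montage, then after a short delay calls PushOverlappingActor.
; EventPushed plays a pushed montage section chosen by GetAnimName from the push origin.
; It temporarily scales max walk speed by the push force, restoring it after the same delay.
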(event EventBeginPlay
  (|CallParentFunction) ; This node is disabled and will not be called.\nDrag off pins to build functionality.
)

(event EventTick
  (params (DeltaSeconds :type Float%20%28single-precision%29))
  (|CallParentFunction DeltaSeconds) ; This node is disabled and will not be called.\nDrag off pins to build functionality.
)

(event EventBeginPush
  (params (Left%20or%20RIght :type Integer))
  ;[1 1 1] Push Other Actor
  (switch int Left%20or%20RIght
    (:0
      (Variables|Default|SetPushDirection "Push_Left"))
    (:1
      (Variables|Default|SetPushDirection "Push_Right")))
  (Animation|PlayAnimMontage "/Game/Characters/Animations/Male/AnimMontage_Male_Push.AnimMontage_Male_Push" 1.0 (Variables|Default|GetPushDirection))
  (Utilities|FlowControl|Delay 0.7)
  (CallFunction|PushOverlappingActor))

(event EventEventPushed
  (params (Pushed%20From :type Name :default "None") (Push%20Force :type Float%20%28single-precision%29))
  (bind _charactermovement (Variables|Character|GetCharacterMovement))
  ;[1 1 1] Pushed by another actor
  (Animation|PlayAnimMontage "/Game/Characters/Animations/Male/AnimMontage_Male_Pushed.AnimMontage_Male_Pushed" 1.0 (CallFunction|GetAnimName Pushed%20From))
  (Variables|Default|SetCharacterWalkSpeed (Variables|/Script/Engine.CharacterMovementComponent|GetMaxWalkSpeed _charactermovement))
  (Variables|/Script/Engine.CharacterMovementComponent|SetMaxWalkSpeed _charactermovement (* Push%20Force (Variables|Default|GetCharacterWalkSpeed)))
  (Utilities|FlowControl|Delay 0.7)
  (Variables|/Script/Engine.CharacterMovementComponent|SetMaxWalkSpeed _charactermovement (Variables|Default|GetCharacterWalkSpeed)))

(fn ConstructionScript
  (|CallParentFunction))