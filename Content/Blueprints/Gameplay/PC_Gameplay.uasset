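; Player controller for a multiplayer runner that manages each player's match state, score, coins and HUDs.
; On local BeginPlay it loads the save, then passes settings and points to GM_Gameplay, which respawns the selected character and tracks scores.
; Events handle the start countdown, pickups with a timed jump boost, pushes, death and the game-over scoreboard.
; Periodic progression scales the character's speed, gravity and jump within clamped limits.
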(event Custom|PassCharacterInfoToServer
  (params (PlayerSettingsInfo :type Structure%20Player%20Info%20Structure))
  ;[1 1 1] Passes character info -- Respawns player with selected character -- Calls SetupChatWindow
  (Variables|Default|SetPlayerSettingsStruct PlayerSettingsInfo)
  (Default|RespawnPlayer (CallFunction|GetGameplayGM) self (.MyPlayerCharacter (Utilities|Struct|BreakStructure_PlayerInfo (Variables|Default|GetPlayerSettingsStruct))))
  (CallFunction|SetupGameplayHUD))

(event Custom|SetupGameplayHUD
  ;[1 1 1] Creates gameplay HUD and adds to viewport
  (bind _returnvalue (UserInterface|CreateWidget "/Game/UI/Blueprints/Gameplay/WB_MainHUD.WB_MainHUD_C"))
  (bind _output_get (Variables|References|SetGameplayHUD _returnvalue))
  (UserInterface|Viewport|AddtoViewport _output_get 0)
  (Class|PlayerController|ActivateTouchInterface))

(event Custom|Actor%20Push
  (params (Left%20or%20RIght :type Integer))
  ;[1 1 1] Apply push from this actor: 1 for right and 0 for left direction
  (Default|BeginPush (Variables|References|GetPlayerCharacter) Left%20or%20RIght))

(event Custom|PassPlayerPointsToServer
  (params (StructPlayerPoints :type Structure%20Player%20Points%20Structure))
  ;[1 1 1] Pass player points info to server
  (Default|UpdatePointsforPlayer (CallFunction|GetGameplayGM) StructPlayerPoints))

(event Custom|GameplayStart
  (bind _playerchar (CallFunction|GetPlayerCharacter))
  ;[1 1 1] Countdown finished - Activate character and begin game
  (Actor|Tick|SetActorTickEnabled _playerchar true)
  (Variables|/Game/Blueprints/Character/BP_Character_Gameplay.BP_Character_Gameplay_C|SetIsInGameplay _playerchar true)
  (Input|SetInputModeGameOnly self))

(event Custom|AddPlayerPointsInfo
  (params (AllPlayers :type Array%20of%20Structure%20Player%20Points%20Structures))
  (bind _gameoverhud (Variables|References|GetGameOverHUD))
  ;[1 1 1] Get all player controllers and add points info -- Update window with info
  (Utilities|IsValid _gameoverhud
    (:Is%20Valid
      (Default|ClearPlayerPoints _gameoverhud)
      (for _array_element AllPlayers
        (Default|UpdatePlayerPointsWindow _gameoverhud (.PlayerName (Utilities|Struct|BreakStructure_PlayerPoints _array_element)) (.PlayerCoins (Utilities|Struct|BreakStructure_PlayerPoints _array_element)) (.PlayerPoints (Utilities|Struct|BreakStructure_PlayerPoints _array_element)))))))

(event Custom|UpdateStartCountdown
  (params (Time%20Remaining :type Float%20%28single-precision%29))
  (bind _gameplayhud (Variables|References|GetGameplayHUD))
  (bind _text_counter (Variables|/Game/UI/Blueprints/Gameplay/WB_MainHUD.WB_MainHUD_C|GetText_Counter _gameplayhud))
  ;[1 1 1] Update game start counter HUD
  (Variables|Countdown|SetRemTime Time%20Remaining)
  (Utilities|IsValid _text_counter
    (:Is%20Valid
      (Rendering|Components|TextRender|SetText _text_counter (Utilities|Text|ToText(Float) (Variables|Countdown|GetRemTime) "HalfToEven" false true 1 324 0 0))
      (if (== (Variables|Countdown|GetRemTime) 0.0)
        (Widget|SetVisibility _text_counter "Collapsed")))))

(event Custom|ShowGameOverHUD
  (params (GameWon :type Boolean))
  (bind _gameplayhud (Variables|References|GetGameplayHUD))
  ;[1 1 1] Show game over HUD
  (Utilities|IsValid _gameplayhud
    (:Is%20Valid
      (Widget|RemovefromParent _gameplayhud)
      (bind _returnvalue (UserInterface|CreateWidget "/Game/UI/Blueprints/Gameplay/WB_GameOver.WB_GameOver_C" self GameWon))
      (bind _output_get (Variables|References|SetGameOverHUD _returnvalue))
      (Class|IHighScoreHUD|UpdateHighScore(Message) _output_get (Variables|CharacterStats|GetHighScore))
      (UserInterface|Viewport|AddtoViewport _output_get 0))))

(event Custom|DisablePlayer
  (params (SimulateBodyFall :type Boolean))
  ;[1 1 1] Call PlayerDeath on server for this PlayerController
  (Default|CharacterDeath (CallFunction|GetPlayerCharacter) SimulateBodyFall))

(event Custom|PointScore
  ;[1 1 1] Add points to this player
  (Variables|CharacterStats|SetScoredPoints (+ (Variables|CharacterStats|GetScoredPoints) (* (Variables|CharacterStats|GetPointsMultiplier) 1)))
  (Class|IHighScoreHUD|UpdatePoints(Message) (Variables|References|GetGameplayHUD) (Variables|CharacterStats|GetScoredPoints))
  (if (Pawn|IsLocalController)
    (CallFunction|PassPlayerPointstoServer (Utilities|Struct|MakeStructure_PlayerPoints (CallFunction|GetPlayerId) (.myplayername (Variables|Default|GetPlayerSettingsStruct)) (Variables|CharacterStats|GetCoins) (Variables|CharacterStats|GetScoredPoints)))))

(event Custom|PeriodicSpeedIncrease
  ;[1 1 1] Increase character movement speed
  (CallFunction|GradualCharacterProgression (CallFunction|GetPlayerCharacter)))

(event Custom|PickUpObject
  (params (ObjectId :type Integer))
  (bind _playerchar (CallFunction|GetPlayerCharacter))
  ;[1 1 1] Exec events based on what PickUps the player collected
  (switch int ObjectId
    (:0
      (Math|Integer|IncrementInt (Variables|CharacterStats|GetCoins)
        (:%20%20
          (Audio|PlaySound2D "/Game/SFX/Pickup_SFX.Pickup_SFX" 1.0 1.0 0.0 0 0))))
    (:1
      (CallFunction|CharacterIncreaseJump _playerchar)
      (Utilities|FlowControl|Delay 6.0)
      (Variables|/Script/Engine.CharacterMovementComponent|SetJumpZVelocity (Variables|/Script/Engine.Character|GetCharacterMovement _playerchar) (Variables|Config|GetDefaultJumpVelocity)))))

(event EventBeginPlay
  ;[1 1 1] Loads player info -- Pass player settings info to server
  (Variables|Default|SetGameStarted true)
  (if (Pawn|IsLocalController)
    (CallFunction|HideLoadingScreen)
    (CallFunction|LoadGame)
    (CallFunction|PassCharacterInfotoServer (Variables|Default|GetPlayerSettingsStruct))
    (CallFunction|PassPlayerPointstoServer (Utilities|Struct|MakeStructure_PlayerPoints (CallFunction|GetPlayerId) (.MyPlayerName (Utilities|Struct|BreakStructure_PlayerInfo (Variables|Default|GetPlayerSettingsStruct))) (Variables|CharacterStats|GetCoins) (Variables|CharacterStats|GetScoredPoints)))))

(fn ConstructionScript)

(fn LoadGame
  (bind _returnvalue (SaveGame|LoadGamefromSlot (Variables|Default|GetPlayerSettingsSave)))
  (bind _asbp_runner_save_game (Utilities|Casting|CastToBP_RunnerSaveGame _returnvalue))
  (Variables|Default|SetPlayerSettingsStruct (Variables|/Game/Blueprints/AllLevels/BP_RunnerSaveGame.BP_RunnerSaveGame_C|GetPlayerSettingsStructure _asbp_runner_save_game))
  (Variables|CharacterStats|SetHighScore (Variables|/Game/Blueprints/AllLevels/BP_RunnerSaveGame.BP_RunnerSaveGame_C|GetHighScore _asbp_runner_save_game)))

(fn GradualCharacterProgression
  (params (PlayerCHaracter :type Character%20Object%20Reference))
  (bind _charactermovement (Variables|/Script/Engine.Character|GetCharacterMovement PlayerCHaracter))
  (Utilities|FlowControl|Sequence
    (:then_0
      (Variables|/Script/Engine.CharacterMovementComponent|SetMaxWalkSpeed _charactermovement (Math|Float|Clamp(Float) (* (Variables|/Script/Engine.CharacterMovementComponent|GetMaxWalkSpeed _charactermovement) (Variables|Config|GetGradualSpeedIncMult)) (Variables|Config|GetMinSpeed) (Variables|Config|GetMaxSpeed))))
    (:then_1
      (Variables|/Script/Engine.CharacterMovementComponent|SetGravityScale _charactermovement (Math|Float|Clamp(Float) (+ (Variables|/Script/Engine.CharacterMovementComponent|GetGravityScale _charactermovement) (Variables|Config|GetGradualGravityIncMult)) 1.3 2.3)))
    (:then_2
      (Variables|/Script/Engine.CharacterMovementComponent|SetJumpZVelocity _charactermovement (Math|Float|Clamp(Float) (* (Variables|/Script/Engine.CharacterMovementComponent|GetJumpZVelocity _charactermovement) (Variables|Config|GetGradualJumpIncMult)) (Variables|Config|GetDefaultJumpVelocity) 1e+03)))))

(fn CharacterIncreaseJump
  (params (PlayerCharacter :type Character%20Object%20Reference))
  (bind _charactermovement (Variables|/Script/Engine.Character|GetCharacterMovement PlayerCharacter))
  (Variables|/Script/Engine.CharacterMovementComponent|SetJumpZVelocity _charactermovement (* (Variables|Config|GetJumpHeightMultiplier) (Variables|/Script/Engine.CharacterMovementComponent|GetJumpZVelocity _charactermovement)))
  (return))

(fn HideLoadingScreen
  (bind _foundwidgets (Widget|GetAllWidgetsOfClass "/Game/UI/Blueprints/AllLevels/WB_LoadingScreen.WB_LoadingScreen_C" true))
  (Widget|RemovefromParent (Utilities|Array|Get(acopy) _foundwidgets)))

(fn GetPlayerCharacter
  (Utilities|IsValid (Variables|References|GetPlayerCharacter)
    (:Is%20Valid
      _)
    (:Is%20Not%20Valid
      (bind _asbp_character_gameplay (Utilities|Casting|CastToBP_Character_Gameplay (Game|GetPlayerCharacter 0)))
      (Variables|References|SetPlayerCharacter _asbp_character_gameplay)))
  (return (Variables|References|GetPlayerCharacter)))

(fn GetGameplayGM
  (Utilities|IsValid (Variables|References|GetGameModeRef)
    (:Is%20Valid
      _)
    (:Is%20Not%20Valid
      (bind _asgm_gameplay (Utilities|Casting|CastToGM_Gameplay (Game|GetGameMode)))
      (Variables|References|SetGameModeRef _asgm_gameplay)))
  (return (Variables|References|GetGameModeRef)))

(fn GetPlayerId
  (if (Networking|IsServer)
    (LocalVariables|SetResultId 0)
    (else
      (LocalVariables|SetResultId 1)))
  (return (LocalVariables|GetResultId)))