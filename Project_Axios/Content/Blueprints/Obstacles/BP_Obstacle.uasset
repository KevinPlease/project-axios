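; Obstacle Blueprint that ends the game for a player whose character hits it.
; On BeginPlay it sets the first child static mesh under the root to block the Pawn channel.
; Hit passes a gameplay character's controller to GameOverForPlayer on GM_Gameplay.
; A DoOnce precedes the character cast, so only the first hit by any actor is evaluated.
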(event Collision|EventHit
  (params (MyComp :type Primitive%20Component%20Object%20Reference) (Other :type Actor%20Object%20Reference) (OtherComp :type Primitive%20Component%20Object%20Reference) (bSelfMoved :type Boolean) (HitLocation :type Vector :default "0, 0, 0") (HitNormal :type Vector :default "0, 0, 0") (NormalImpulse :type Vector :default "0, 0, 0") (Hit :type Hit%20Result%20Structure%20%28by%20ref%29))
  ;[1 1 1] Check if Hit by character player and call Player Death on the player controller
  (Utilities|FlowControl|DoOnce false
    (:Completed
      (bind _asbp_character_gameplay (Utilities|Casting|CastToBP_Character_Gameplay Other)) ; Check if other actor is our character
      (bind _asgm_gameplay (Utilities|Casting|CastToGM_Gameplay (Game|GetGameMode)))
      (bind _aspc_gameplay (Utilities|Casting|CastToPC_Gameplay (Pawn|GetController _asbp_character_gameplay)))
      (Default|GameOverforPlayer _asgm_gameplay _aspc_gameplay))))

(event EventBeginPlay
  ;[1 1 1] Dynamically change collision for the Static Mesh attached with this Blueprint
  (bind _asstatic_mesh_component (Utilities|Casting|CastToStaticMeshComponent (Components|GetChildComponent (Variables|Default|GetDefaultSceneRoot) 0)))
  (Collision|SetCollisionResponsetoChannel _asstatic_mesh_component "ECC_Pawn" "ECR_Block"))

(fn ConstructionScript)