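; Master track tile for an endless runner that fills three lanes with random obstacles and pickups.
; On BeginPlay, once the game mode's InitialCount reaches two, each lane rerolls per range check to spawn a pipe, box, power pickup, boots or nothing.
; While the game runs, player overlap with the end box requests the next tile, updates score and speed, then after a delay destroys this tile and its visible spawned actors.
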(event OnComponentBeginOverlap(Box)
  (params (OverlappedComponent :type Primitive%20Component%20Object%20Reference) (OtherActor :type Actor%20Object%20Reference) (OtherComp :type Primitive%20Component%20Object%20Reference) (OtherBodyIndex :type Integer) (bFromSweep :type Boolean) (SweepResult :type Hit%20Result%20Structure%20%28by%20ref%29))
  ;[1 1 1] On End of Tile Reached Spawn Next TIle AND Destroy Previous
  (if (CallFunction|IsinGame)
    (Utilities|Casting|CastToBP_Character_Gameplay OtherActor)
    (Default|SpawnTile (Variables|References|GetGameModeRef))
    (bind _aspc_gameplay (Utilities|Casting|CastToPC_Gameplay (Game|GetPlayerController 0)))
    (Default|PointScore _aspc_gameplay)
    (Default|PeriodicSpeedIncrease _aspc_gameplay)
    (Utilities|FlowControl|Delay 0.5)
    (CallFunction|CleanUpActors)))

(event EventBeginPlay
  ;[1 1 1] Begin Play
  (bind _asgm_gameplay (Utilities|Casting|CastToGM_Gameplay (Game|GetGameMode)))
  (Variables|References|SetGameModeRef _asgm_gameplay)
  (bind _asbp_character_gameplay (Utilities|Casting|CastToBP_Character_Gameplay (Game|GetPlayerCharacter 0)))
  (Variables|References|SetThirdPersonCharacter _asbp_character_gameplay)
  (if (>= (Variables|/Game/Blueprints/Gameplay/GM_Gameplay.GM_Gameplay_C|GetInitialCount (Variables|References|GetGameModeRef)) 2)
    (CallFunction|SpawnObstacles)))

(fn ConstructionScript)

(fn SpawnObstacles
  (bind _returnvalue (Math|Random|RandomFloatinRange 0.0 2.0))
  (bind _returnvalue_2 (Math|Random|RandomFloatinRange 0.0 2.0))
  (bind _returnvalue_3 (Math|Random|RandomFloatinRange 0.0 2.0))
  (bind _right (Variables|Default|GetRight))
  (bind _left (Variables|Default|GetLeft))
  (bind _center (Variables|Default|GetCenter))
  (bind _returnvalue_4 (Transformation|GetWorldTransform _right))
  (bind _returnvalue_5 (Transformation|GetWorldTransform _left))
  (bind _returnvalue_6 (Transformation|GetWorldTransform _center))
  (Utilities|FlowControl|Sequence
    (:then_0
      ;[1 1 1] Left Lane
      (if (Math|Float|InRange(Float) _returnvalue 0.0 0.5 true false)
        (bind _returnvalue_7 (Game|SpawnActorfromClass "/Game/Blueprints/Obstacles/BP_Obstacle_Pipe.BP_Obstacle_Pipe_C" _returnvalue_5 "Undefined" 0 0))
        (Utilities|Array|Add (Variables|Default|GetObjectsToDestroy) _returnvalue_7)
        (elif (Math|Float|InRange(Float) _returnvalue 0.5 0.65 true false)
          (bind _returnvalue_8 (Game|SpawnActorfromClass "/Game/Blueprints/Obstacles/BP_Obstacle_Box.BP_Obstacle_Box_C" _returnvalue_5 "Undefined" 0 0))
          (Utilities|Array|Add (Variables|Default|GetObjectsToDestroy) _returnvalue_8)
          (elif (Math|Float|InRange(Float) _returnvalue 0.65 0.9 true false)
            (bind _returnvalue_9 (Game|SpawnActorfromClass "/Game/Blueprints/Pickups/BP_Pickup_Power.BP_Pickup_Power_C" _returnvalue_5 "Undefined" 0 0))
            (Utilities|Array|Add (Variables|Default|GetObjectsToDestroy) _returnvalue_9)
            (elif (Math|Float|InRange(Float) _returnvalue 0.9 1.0)
              (bind _returnvalue_10 (Game|SpawnActorfromClass "/Game/Blueprints/Pickups/BP_Pickup_Boots.BP_Pickup_Boots_C" _returnvalue_5 "Undefined" 0 0))
              (Utilities|Array|Add (Variables|Default|GetObjectsToDestroy) _returnvalue_10))))))
    (:then_1
      ;[1 1 1] Center Lane
      (if (Math|Float|InRange(Float) _returnvalue_2 0.0 0.5 true false)
        (bind _returnvalue_11 (Game|SpawnActorfromClass "/Game/Blueprints/Obstacles/BP_Obstacle_Pipe.BP_Obstacle_Pipe_C" _returnvalue_6 "Undefined" 0 0))
        (Utilities|Array|Add (Variables|Default|GetObjectsToDestroy) _returnvalue_11)
        (elif (Math|Float|InRange(Float) _returnvalue_2 0.5 0.65 true false)
          (bind _returnvalue_12 (Game|SpawnActorfromClass "/Game/Blueprints/Obstacles/BP_Obstacle_Box.BP_Obstacle_Box_C" _returnvalue_6 "Undefined" 0 0))
          (Utilities|Array|Add (Variables|Default|GetObjectsToDestroy) _returnvalue_12)
          (elif (Math|Float|InRange(Float) _returnvalue_2 0.65 0.9 true false)
            (bind _returnvalue_13 (Game|SpawnActorfromClass "/Game/Blueprints/Pickups/BP_Pickup_Power.BP_Pickup_Power_C" _returnvalue_6 "Undefined" 0 0))
            (Utilities|Array|Add (Variables|Default|GetObjectsToDestroy) _returnvalue_13)
            (elif (Math|Float|InRange(Float) _returnvalue_2 0.9 1.0)
              (bind _returnvalue_14 (Game|SpawnActorfromClass "/Game/Blueprints/Pickups/BP_Pickup_Boots.BP_Pickup_Boots_C" _returnvalue_6 "Undefined" 0 0))
              (Utilities|Array|Add (Variables|Default|GetObjectsToDestroy) _returnvalue_14))))))
    (:then_2
      ;[1 1 1] Left Lane
      (if (Math|Float|InRange(Float) _returnvalue_3 0.0 0.5 true false)
        (bind _returnvalue_15 (Game|SpawnActorfromClass "/Game/Blueprints/Obstacles/BP_Obstacle_Pipe.BP_Obstacle_Pipe_C" _returnvalue_4 "Undefined" 0 0))
        (Utilities|Array|Add (Variables|Default|GetObjectsToDestroy) _returnvalue_15)
        (elif (Math|Float|InRange(Float) _returnvalue_3 0.5 0.65 true false)
          (bind _returnvalue_16 (Game|SpawnActorfromClass "/Game/Blueprints/Obstacles/BP_Obstacle_Box.BP_Obstacle_Box_C" _returnvalue_4 "Undefined" 0 0))
          (Utilities|Array|Add (Variables|Default|GetObjectsToDestroy) _returnvalue_16)
          (elif (Math|Float|InRange(Float) _returnvalue_3 0.65 0.9 true false)
            (bind _returnvalue_17 (Game|SpawnActorfromClass "/Game/Blueprints/Pickups/BP_Pickup_Power.BP_Pickup_Power_C" _returnvalue_4 "Undefined" 0 0))
            (Utilities|Array|Add (Variables|Default|GetObjectsToDestroy) _returnvalue_17)
            (elif (Math|Float|InRange(Float) _returnvalue_3 0.9 1.0)
              (bind _returnvalue_18 (Game|SpawnActorfromClass "/Game/Blueprints/Pickups/BP_Pickup_Boots.BP_Pickup_Boots_C" _returnvalue_4 "Undefined" 0 0))
              (Utilities|Array|Add (Variables|Default|GetObjectsToDestroy) _returnvalue_18))))))))

(fn CleanUpActors
  (if (CallFunction|IsinGame)
    (Actor|DestroyActor)
    ;[1 1 1] Destroy all previous actors
    (if (> (Utilities|Array|Length (Variables|Default|GetObjectsToDestroy)) 0)
      (for _array_element (Variables|Default|GetObjectsToDestroy)
        (Utilities|IsValid _array_element
          (:Is%20Valid
            (if (Variables|/Script/Engine.SceneComponent|GetbVisible (Components|GetChildComponent (Variables|/Script/Engine.Actor|GetRootComponent _array_element) 0))
              (Actor|DestroyActor _array_element)))))
      ;[1 1 1] Reset the List when all actors are destroyed
      (Utilities|Array|Clear (Variables|Default|GetObjectsToDestroy)))))

(fn IsinGame
  (return (not (Variables|/Game/Blueprints/Gameplay/GM_Gameplay.GM_Gameplay_C|GetGameOver (Variables|References|GetGameModeRef)))))