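; Player character for a runner game that auto-runs along control yaw during gameplay, with strafe input and swipe up/down to jump or slam down.
; BeginPlay enables the auto-run Tick from the controller's GameStarted flag, or the game mode if that cast fails.
; Z/X play directional push montages, then shove an overlapping character on that side, temporarily scaling its walk speed.
; CharacterDeath ragdolls and switches to UI input; its high-score save logic is unconnected.
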(event Custom|Event%20Pushed
  (params (Pushed%20From :type Name) (Push%20Force :type Float%20%28single-precision%29))
  (bind _charactermovement (Variables|Character|GetCharacterMovement))
  ;[1 1 1] Push this actor by an offset vector multiplied by a push force
  (Animation|PlayAnimMontage "/Game/Mannequin/Animations/Pushed_Anim_Montage.Pushed_Anim_Montage" 1.0 (CallFunction|GetAnimName Pushed%20From))
  (Variables|MyCharacter|SetCharacterWalkSpeed (Variables|/Script/Engine.CharacterMovementComponent|GetMaxWalkSpeed _charactermovement))
  (Variables|/Script/Engine.CharacterMovementComponent|SetMaxWalkSpeed _charactermovement (* Push%20Force (Variables|MyCharacter|GetCharacterWalkSpeed)))
  (Utilities|FlowControl|Delay 0.7)
  (Variables|/Script/Engine.CharacterMovementComponent|SetMaxWalkSpeed _charactermovement (Variables|MyCharacter|GetCharacterWalkSpeed)))

(event Custom|Begin%20Push
  (params (Left%20or%20RIght :type Integer))
  ;[1 1 1] Push Character - Play Animation & Check for actors to push
  (switch int Left%20or%20RIght
    (:0
      (Variables|MyCharacter|SetPushDirection "Push_Left"))
    (:1
      (Variables|MyCharacter|SetPushDirection "Push_Right")))
  (Animation|PlayAnimMontage "/Game/Mannequin/Animations/Push_AnimMontage.Push_AnimMontage" 1.0 (Variables|MyCharacter|GetPushDirection))
  (Utilities|FlowControl|Delay 0.7)
  (CallFunction|PushOverlappingActor))

(event EventTick
  (params (DeltaSeconds :type Float%20%28single-precision%29))
  ;[1 1 1] Movement input - Checks if in gameplay and splits movement logic vs "swipe to move"
  (Pawn|Input|AddMovementInput (Math|Vector|GetForwardVector (Math|Rotator|MakeRotator 0.0 0.0 (.Yaw (Math|Rotator|BreakRotator (Pawn|GetControlRotation :!class /Script/Engine.Pawn))))) 1.0 false))

(event EventBeginPlay
  ;[1 1 1] TODO: Needs to be revised: Checks when gameplay has begun for both server and client separately
  (bind _aspc_gameplay (Utilities|Casting|CastToPC_Gameplay (Game|GetPlayerController 0))
    (:then
      (Actor|Tick|SetActorTickEnabled (Variables|/Game/Blueprints/Gameplay/PC_Gameplay.PC_Gameplay_C|GetGameStarted _aspc_gameplay)))
    (:CastFailed
      (Utilities|Casting|CastToGM_Gameplay (Game|GetGameMode))
      (Actor|Tick|SetActorTickEnabled true)))
  (Variables|Default|SetIsInGameplay (Class|Actor|IsActorTickEnabled)))

(event Input|AxisEvents|InputAxisMoveRight
  (params (AxisValue :type Float%20%28single-precision%29))
  ;[1 1 1] Movement input - Checks if in gameplay and splits movement logic vs "swipe to move"
  (Pawn|Input|AddMovementInput (Math|Vector|GetRightVector (Math|Rotator|MakeRotator 0.0 0.0 (.Yaw (Math|Rotator|BreakRotator (Pawn|GetControlRotation :!class /Script/Engine.Pawn))))) AxisValue false))

(event Input|AxisEvents|InputAxisMoveForward
  (params (AxisValue :type Float%20%28single-precision%29))
  ;[1 1 1] Movement input - Checks if in gameplay and splits movement logic vs "swipe to move"
  (if (not (Variables|Default|GetIsInGameplay))
    (Pawn|Input|AddMovementInput (Math|Vector|GetForwardVector (Math|Rotator|MakeRotator 0.0 0.0 (.Yaw (Math|Rotator|BreakRotator (Pawn|GetControlRotation :!class /Script/Engine.Pawn))))) AxisValue false)))

(event Input|KeyboardEvents|X
  (params (Key :type Key%20Structure))
  ;[1 1 1] Keyboard Input for Pushing Left/Right
  (:Pressed
    (CallFunction|BeginPush 1)))

(event Input|KeyboardEvents|Z
  (params (Key :type Key%20Structure))
  ;[1 1 1] Keyboard Input for Pushing Left/Right
  (:Pressed
    (CallFunction|BeginPush)))

(event Input|TouchEvents|InputTouch
  (params (Location :type Vector) (FingerIndex :type ETouchIndex%20Enum))
  (bind _returnvalue (CallFunction|GetTouchLocation))
  ;[1 1 1] Swipe Controls
  (:Pressed
    (Variables|Default|SetIsPressed true)
    (Variables|Default|SetTouchStart2D _returnvalue))
  (:Released
    (Variables|Default|SetIsPressed false)
    (if (> (Math|Vector2D|Vector2DLength (- (Variables|Default|GetTouchStart2D) _returnvalue)) 1e+02)
      (Utilities|FlowControl|Sequence
        (:then_0
          (Utilities|FlowControl|DoOnce false :!label _label
            (:Completed
              (Variables|Default|SetTouchEnd2D _returnvalue)
              (switch string (CallFunction|GetFinalSwipeDirection (Variables|Default|GetTouchStart2D) (Variables|Default|GetTouchEnd2D))
                (:Up
                  (Character|Jump))
                (:Down
                  (Physics|AddImpulse (Variables|Character|GetCharacterMovement) "0, 0,-3000.000000" true))))))
        (:then_1
          (Utilities|FlowControl|Delay 0.5)
          (goto _label Reset))))))

(fn ConstructionScript)

(fn CharacterDeath
  (Utilities|FlowControl|Sequence
    (:then_0
      ;[1 1 1] Death Anim. purposes
      (Physics|SetSimulatePhysics (Variables|Character|GetMesh) true)
      (Pawn|Components|CharacterMovement|DisableMovement (Variables|Character|GetCharacterMovement))
      (Input|SetInputModeUIOnly (Game|GetPlayerController 0) 0 "DoNotLock"))))

(fn GetMyGameMode
  (Utilities|IsValid (Variables|References|GetGameModeRef)
    (:Is%20Valid
      _)
    (:Is%20Not%20Valid
      (bind _asgm_gameplay (Utilities|Casting|CastToGM_Gameplay (Game|GetGameMode)))
      (Variables|References|SetGameModeRef _asgm_gameplay)))
  (return (Variables|References|GetGameModeRef)))

(fn PushOverlappingActor
  ;[1 1 1] Check for valid character in radius && Compare location to find direction of push && Commit push
  (bind _asbp_character_gameplay (Utilities|Casting|CastToBP_Character_Gameplay (Utilities|Array|Get(acopy) (Collision|GetOverlappingActors (Variables|Default|GetPushCapsule) "BP_Character_Gameplay_C" :!class /Script/Engine.PrimitiveComponent) 1)))
  (Math|Float|CompareFloat (.y (Transformation|GetActorLocation _asbp_character_gameplay)) (.y (Transformation|GetActorLocation))
    (:>
      (LocalVariables|SetPushedActorLocation "Push_Right"))
    (:<
      (LocalVariables|SetPushedActorLocation "Push_Left")))
  (if (Utilities|Enum|Equal(Enum) (LocalVariables|GetPushedActorLocation) (Utilities|String|ToString(Name) (Variables|MyCharacter|GetPushDirection)))
    (CallFunction|EventPushed _asbp_character_gameplay (Variables|MyCharacter|GetPushDirection) (Variables|Stats|GetStatPushForce))))

(fn GetTouchLocation
  (bind _returnvalue (Game|GetPlayerController 0))
  (bind (_locationx _locationy) (Class|PlayerController|GetInputTouchState _returnvalue "Touch1"))
  (return (Math|Vector2D|MakeVector2D _locationx _locationy)))

(fn GetFinalSwipeDirection
  (params (TouchStart :type Vector%202D%20Structure) (TouchEnd :type Vector%202D%20Structure))
  (bind _returnvalue (- TouchStart TouchEnd))
  (if (> (Math|Float|Absolute(Float) (.x _returnvalue)) (Math|Float|Absolute(Float) (.y _returnvalue)))
    (if (> (.x _returnvalue) 0.0)
      (LocalVariables|SetSwipeDir "Left")
      (else
        (LocalVariables|SetSwipeDir "Right")))
    (elif (> (.y _returnvalue) 0.0)
      (LocalVariables|SetSwipeDir "Up")
      (else
        (LocalVariables|SetSwipeDir "Down"))))
  (return (LocalVariables|GetSwipeDir)))

(fn GetAnimName
  (params (From%20Push%20Anim%20Name :type Name))
  (switch name From%20Push%20Anim%20Name
    (:Push_Left
      (LocalVariables|SetAnim%20Montage "Pushed_From_Left"))
    (:Push_Right
      (LocalVariables|SetAnim%20Montage "Pushed_From_Right")))
  (return (LocalVariables|GetAnim%20Montage)))