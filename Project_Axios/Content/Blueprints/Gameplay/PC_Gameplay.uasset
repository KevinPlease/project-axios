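; Player controller for a runner game, handling player setup, score, pickups and HUDs.
; On local BeginPlay it loads saved settings and passes them on to GM_Gameplay, which respawns the selected character, then creates the main HUD.
; It swaps in win or loss screens and forwards deaths to the game mode.
; It also applies clamped speed increases, counts coins, grants timed jump boosts and relays pushes to the character.
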(event Custom|PassCharacterInfoToServer
  (params (PlayerSettingsInfo :type Structure%20Player%20Info%20Structure))
  ;[1 1 1] Passes character info -- Respawns player with selected character -- Calls SetupChatWindow
  (Variables|Default|SetPlayerSettings PlayerSettingsInfo)
  (bind _asgm_gameplay (Utilities|Casting|CastToGM_Gameplay (Game|GetGameMode)))
  (Default|RespawnPlayer _asgm_gameplay self (.MyPlayerCharacter (Utilities|Struct|BreakStructure_PlayerInfo (Variables|Default|GetPlayerSettings))))
  (CallFunction|SetupGameplayHUD))

(event Custom|SetupGameplayHUD
  ;[1 1 1] Creates gameplay HUD and adds to viewport
  (bind _returnvalue (UserInterface|CreateWidget "/Game/UI/Blueprints/Gameplay/WB_MainHUD.WB_MainHUD_C"))
  (bind _output_get (Variables|References|SetGameplayHUD _returnvalue))
  (UserInterface|Viewport|AddtoViewport _output_get 0)
  (Class|PlayerController|ActivateTouchInterface))

(event Custom|Actor%20Push
  (params (Left%20or%20RIght :type Integer))
  ;[1 1 1] Apply push from this actor: 1 for right and 0 for left direction
  (Default|BeginPush (Variables|References|GetPlayerCharacter) Left%20or%20RIght))

(event Custom|ShowGameLostHUD
  (bind _gameplayhud (Variables|References|GetGameplayHUD))
  ;[1 1 1] Show Game Over UI on PlayerDeath
  (Utilities|IsValid _gameplayhud
    (:Is%20Valid
      (Widget|RemovefromParent _gameplayhud)
      (bind _returnvalue (UserInterface|CreateWidget "/Game/UI/Blueprints/Gameplay/WB_GameOver_Lost.WB_GameOver_Lost_C" self))
      (bind _output_get (Variables|References|SetGameOverHUD _returnvalue))
      (UserInterface|Viewport|AddtoViewport _output_get 0))))

(event Custom|ShowGameWonHUD
  (bind _gameplayhud (Variables|References|GetGameplayHUD))
  ;[1 1 1] Show game win HUD
  (Utilities|IsValid _gameplayhud
    (:Is%20Valid
      (Widget|RemovefromParent _gameplayhud)
      (bind _returnvalue (UserInterface|CreateWidget "/Game/UI/Blueprints/Gameplay/WB_GameOver_Win.WB_GameOver_Win_C" self))
      (bind _output_get (Variables|References|SetGameOverHUD _returnvalue))
      (UserInterface|Viewport|AddtoViewport _output_get 0))))

(event Custom|PlayerDeath
  ;[1 1 1] Call PlayerDeath on server for this PlayerController
  (bind _asgm_gameplay (Utilities|Casting|CastToGM_Gameplay (Game|GetGameMode)))
  (Default|PlayerDeath _asgm_gameplay self))

(event Custom|PointScore
  ;[1 1 1] Add points to this player
  (Variables|CharacterStats|SetScoredPoints (+ (Variables|CharacterStats|GetScoredPoints) (* (Variables|CharacterStats|GetPointsMultiplier) 1))))

(event Custom|PeriodicSpeedIncrease
  ;[1 1 1] Increase character movement speed
  (Utilities|IsValid (Variables|References|GetPlayerCharacter)
    (:Is%20Valid
      _)
    (:Is%20Not%20Valid
      (bind _asbp_character_gameplay (Utilities|Casting|CastToBP_Character_Gameplay (Game|GetPlayerCharacter 0)))
      (Variables|References|SetPlayerCharacter _asbp_character_gameplay)))
  (CallFunction|CharacterIncreaseSpeed (Variables|References|GetPlayerCharacter)))

(event Custom|PickUpObject
  (params (ObjectId :type Integer))
  ;[1 1 1] Exec events based on what PickUps the player collected
  (switch int ObjectId
    (:0
      (Math|Integer|IncrementInt (Variables|CharacterStats|GetCoins)
        (:%20%20
          (Audio|PlaySound2D "/Game/SFX/Pickup_SFX.Pickup_SFX" 1.0 1.0 0.0 0 0))))
    (:1
      (Utilities|IsValid (Variables|References|GetPlayerCharacter)
        (:Is%20Valid
          (CallFunction|CharacterIncreaseJump (Variables|References|GetPlayerCharacter))
          (Utilities|FlowControl|Delay 1e+01)
          (Variables|/Script/Engine.CharacterMovementComponent|SetJumpZVelocity (Variables|/Script/Engine.Character|GetCharacterMovement (Variables|References|GetPlayerCharacter)) (Variables|CharacterStats|GetDefaultJumpVelocity)))
        (:Is%20Not%20Valid
          (bind _asbp_character_gameplay (Utilities|Casting|CastToBP_Character_Gameplay (Game|GetPlayerCharacter 0)))
          (Variables|References|SetPlayerCharacter _asbp_character_gameplay))))))

(event EventBeginPlay
  ;[1 1 1] Loads player info -- Pass player settings info to server
  (Variables|Default|SetGameStarted true)
  (if (Pawn|IsLocalController)
    (CallFunction|HideLoadingScreen)
    (CallFunction|LoadGame)
    (CallFunction|PassCharacterInfotoServer (Variables|Default|GetPlayerSettings))))

(fn ConstructionScript)

(fn LoadGame
  (bind _returnvalue (SaveGame|LoadGamefromSlot (Variables|Default|GetPlayerSettingsSave)))
  (bind _asbp_runner_save_game (Utilities|Casting|CastToBP_RunnerSaveGame _returnvalue))
  (Variables|Default|SetPlayerSettings (Variables|/Game/Blueprints/AllLevels/BP_RunnerSaveGame.BP_RunnerSaveGame_C|GetStruct_PlayerInfo _asbp_runner_save_game)))

(fn CharacterIncreaseSpeed
  (params (PlayerCHaracter :type Character%20Object%20Reference))
  (bind _charactermovement (Variables|/Script/Engine.Character|GetCharacterMovement PlayerCHaracter))
  (Variables|/Script/Engine.CharacterMovementComponent|SetMaxWalkSpeed _charactermovement (Math|Float|Clamp(Float) (* (Variables|/Script/Engine.CharacterMovementComponent|GetMaxWalkSpeed _charactermovement) (Variables|CharacterStats|GetGradualSpeedIncreaseMultiplier)) (Variables|CharacterStats|GetMinSpeed) (Variables|CharacterStats|GetMaxSpeed))))

(fn CharacterIncreaseJump
  (params (PlayerCharacter :type Character%20Object%20Reference))
  (bind _charactermovement (Variables|/Script/Engine.Character|GetCharacterMovement PlayerCharacter))
  (Variables|/Script/Engine.CharacterMovementComponent|SetJumpZVelocity _charactermovement (* (Variables|CharacterStats|GetJumpHeightMultiplier) (Variables|/Script/Engine.CharacterMovementComponent|GetJumpZVelocity _charactermovement)))
  (return))

(fn HideLoadingScreen
  (bind _foundwidgets (Widget|GetAllWidgetsOfClass "/Game/UI/Blueprints/AllLevels/WB_LoadingScreen.WB_LoadingScreen_C" true))
  (Widget|RemovefromParent (Utilities|Array|Get(acopy) _foundwidgets)))